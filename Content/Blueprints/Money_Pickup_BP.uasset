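; Money pickup actor that rewards the side-scroller player character with cash.
; It spins around its vertical axis every tick by a fixed yaw step, independent of frame time.
; When the character overlaps its Box, it shows a configurable message, adds a hard-coded money amount to that character and destroys itself.
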(event `self.ReceiveTick`
  (params (DeltaSeconds :type "Float (single-precision)"))
  (`self.K2_SetActorRotation` (`KismetMathLibrary.MakeRotator` (.roll (`self.K2_GetActorRotation`)) (.pitch (`self.K2_GetActorRotation`)) (+ (.yaw (`self.K2_GetActorRotation`)) 3.0))))

(event `self.Box.OnComponentBeginOverlap`
  (params (OverlappedComponent :type "PrimitiveComponent Object Reference") (OtherActor :type "Actor Object Reference") (OtherComp :type "PrimitiveComponent Object Reference") (OtherBodyIndex :type Integer) (bFromSweep :type Boolean) (SweepResult :type "HitResult Structure (by ref)"))
  (bind _asbp_side_scroller_character (cast `/Game/2DSideScroller/Blueprints/BP_SideScrollerCharacter` OtherActor))
  (`/Game/2DSideScroller/Blueprints/BP_SideScrollerCharacter.Display Message` _asbp_side_scroller_character (`self.Duration`) (`self.Display Text`))
  (`/Game/2DSideScroller/Blueprints/BP_SideScrollerCharacter.Add Money` _asbp_side_scroller_character 5900)
  (`self.K2_DestroyActor`))

(fn `UserConstructionScript`)