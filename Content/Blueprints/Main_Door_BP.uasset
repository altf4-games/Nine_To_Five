(event `self.Box.OnComponentBeginOverlap`
  (params (OverlappedComponent :type "PrimitiveComponent Object Reference") (OtherActor :type "Actor Object Reference") (OtherComp :type "PrimitiveComponent Object Reference") (OtherBodyIndex :type Integer) (bFromSweep :type Boolean) (SweepResult :type "HitResult Structure (by ref)"))
  ;[1 1 1] Door TP
  (bind _asbp_side_scroller_character (cast `/Game/2DSideScroller/Blueprints/BP_SideScrollerCharacter` OtherActor))
  (if (>= (`/Game/2DSideScroller/Blueprints/BP_SideScrollerCharacter.Time` _asbp_side_scroller_character) 17)
    (`/Game/2DSideScroller/Blueprints/BP_SideScrollerCharacter.Display Message` _asbp_side_scroller_character 8.0 "Press E To Leave")
    (`self.EnableInput` (`PlayerState.GetPlayerController` (`Pawn.PlayerState` _asbp_side_scroller_character)))))

(event `Key|E`
  (params (Key :type "Key Structure"))
  ;[1 1 1] Door TP
  (:`Pressed`
    (bind _asbp_side_scroller_character (cast `/Game/2DSideScroller/Blueprints/BP_SideScrollerCharacter` (`GameplayStatics.GetPlayerCharacter` 0)))
    (`/Game/2DSideScroller/Blueprints/BP_SideScrollerCharacter.Display Message` _asbp_side_scroller_character 5.0 "End of Demo: Thanks for playing")
    (`KismetSystemLibrary.Delay` 5.0)
    (`GameplayStatics.OpenLevelBySoftObjectPtr` "/Game/Maps/MM.MM")))

(fn `UserConstructionScript`)