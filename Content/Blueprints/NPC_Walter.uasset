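; NPC Walter is a side-scroller NPC that offers the player a one-time lab session.
; Its sphere overlap checks for a Lab Coat, then either prompts and enables E input, or shows the NPC's subtitle and sets HasLabCoat despite the missing coat.
; Pressing E plays a sound and, unless both LabGiven and HasLabCoat are set, marks the lab given, updates time and shows a delayed quip.
; Leaving the sphere disables input.
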(event `self.Sphere.OnComponentBeginOverlap`
  (params (OverlappedComponent :type "PrimitiveComponent Object Reference") (OtherActor :type "Actor Object Reference") (OtherComp :type "PrimitiveComponent Object Reference") (OtherBodyIndex :type Integer) (bFromSweep :type Boolean) (SweepResult :type "HitResult Structure (by ref)"))
  (if (not (`self.LabGiven`))
    (bind _asbp_side_scroller_character (cast `/Game/2DSideScroller/Blueprints/BP_SideScrollerCharacter` OtherActor))
    (if (`KismetArrayLibrary.Array_Contains` (`/Game/2DSideScroller/Blueprints/BP_SideScrollerCharacter.Inventory` _asbp_side_scroller_character) "Lab Coat")
      (`/Game/2DSideScroller/Blueprints/BP_SideScrollerCharacter.Display Message` _asbp_side_scroller_character 10.0 "Press E To Attend Lab Session")
      (`self.EnableInput` (`GameplayStatics.GetPlayerController` 0))
      (else
        (`/Game/2DSideScroller/Blueprints/BP_SideScrollerCharacter.Display Subtitle` _asbp_side_scroller_character (`self.Duration`) (`KismetTextLibrary.Conv_StringToText` (`KismetStringLibrary.Concat_StrStr` (`self.Name`) ": " (`self.Subtitle`))))
        (set `self.HasLabCoat` true)))))

(event `Key|E`
  (params (Key :type "Key Structure"))
  (:`Pressed`
    (`GameplayStatics.PlaySound2D` "/Game/Audio/hitHurt.hitHurt" 1.0 1.0 0.0 null null)
    (if (not (and (`self.LabGiven`) (`self.HasLabCoat`)))
      (set `self.LabGiven` true)
      (bind _asbp_side_scroller_character (cast `/Game/2DSideScroller/Blueprints/BP_SideScrollerCharacter` (`GameplayStatics.GetPlayerCharacter` 0)))
      (`/Game/2DSideScroller/Blueprints/BP_SideScrollerCharacter.UpdateTime` _asbp_side_scroller_character 2)
      (`KismetSystemLibrary.Delay` 1.0)
      (`/Game/2DSideScroller/Blueprints/BP_SideScrollerCharacter.Display Subtitle` _asbp_side_scroller_character 5.0 "You: Who let sir cook"))))

(event `self.Sphere.OnComponentEndOverlap`
  (params (OverlappedComponent :type "PrimitiveComponent Object Reference") (OtherActor :type "Actor Object Reference") (OtherComp :type "PrimitiveComponent Object Reference") (OtherBodyIndex :type Integer))
  (`self.DisableInput` (`GameplayStatics.GetPlayerController` 0)))

(fn `UserConstructionScript`)