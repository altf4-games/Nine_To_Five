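; NPC cafe vendor to whom the side-scroller player can repay a debt, once.
; Entering its sphere shows the NPC's named subtitle and a key prompt and enables input on the actor; leaving disables it.
; Pressing E with enough money sets DebtGiven, advances the character's time, deducts the payment and shows a delayed player reply.
; DebtGiven blocks repeat prompts and payments; insufficient money gets no feedback.
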(event `self.Sphere.OnComponentBeginOverlap`
  (params (OverlappedComponent :type "PrimitiveComponent Object Reference") (OtherActor :type "Actor Object Reference") (OtherComp :type "PrimitiveComponent Object Reference") (OtherBodyIndex :type Integer) (bFromSweep :type Boolean) (SweepResult :type "HitResult Structure (by ref)"))
  (if (not (`self.DebtGiven`))
    (bind _asbp_side_scroller_character (cast `/Game/2DSideScroller/Blueprints/BP_SideScrollerCharacter` OtherActor))
    (`/Game/2DSideScroller/Blueprints/BP_SideScrollerCharacter.Display Subtitle` _asbp_side_scroller_character (`self.Duration`) (`KismetTextLibrary.Conv_StringToText` (`KismetStringLibrary.Concat_StrStr` (`self.Name`) ": " (`self.Subtitle`))))
    (`/Game/2DSideScroller/Blueprints/BP_SideScrollerCharacter.Display Message` _asbp_side_scroller_character 10.0 "Press E To Payback 6000 Debt")
    (`self.EnableInput` (`GameplayStatics.GetPlayerController` 0))))

(event `Key|E`
  (params (Key :type "Key Structure"))
  (:`Pressed`
    (bind _asbp_side_scroller_character (cast `/Game/2DSideScroller/Blueprints/BP_SideScrollerCharacter` (`GameplayStatics.GetPlayerCharacter` 0)))
    (if (>= (`/Game/2DSideScroller/Blueprints/BP_SideScrollerCharacter.Money` _asbp_side_scroller_character) 6000)
      (if (not (`self.DebtGiven`))
        (set `self.DebtGiven` true)
        (bind _asbp_side_scroller_character_2 (cast `/Game/2DSideScroller/Blueprints/BP_SideScrollerCharacter` (`GameplayStatics.GetPlayerCharacter` 0)))
        (`/Game/2DSideScroller/Blueprints/BP_SideScrollerCharacter.UpdateTime` _asbp_side_scroller_character_2 2)
        (`/Game/2DSideScroller/Blueprints/BP_SideScrollerCharacter.Add Money` _asbp_side_scroller_character_2 -6000)
        (`KismetSystemLibrary.Delay` 1.0)
        (`/Game/2DSideScroller/Blueprints/BP_SideScrollerCharacter.Display Subtitle` _asbp_side_scroller_character_2 5.0 "You: Now give ten plate samosas")))))

(event `self.Sphere.OnComponentEndOverlap`
  (params (OverlappedComponent :type "PrimitiveComponent Object Reference") (OtherActor :type "Actor Object Reference") (OtherComp :type "PrimitiveComponent Object Reference") (OtherBodyIndex :type Integer))
  (`self.DisableInput` (`GameplayStatics.GetPlayerController` 0)))

(fn `UserConstructionScript`)